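; Behavior tree task that picks a random patrol destination for an EnemyCharacter.
; It draws a debug sphere of the patrol radius and sets the patrol walk speed.
; It writes a random reachable point within that radius to the patrol location blackboard key, falling back to the enemy's current location.
; It finishes successfully, or fails if the pawn is not an EnemyCharacter.
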(event EventReceiveExecuteAI
  (params (OwnerController :type AI%20Controller%20Object%20Reference) (ControlledPawn :type Pawn%20Object%20Reference))
  (bind _patrolradius (Variables|Default|GetPatrolRadius))
  (bind _patrollocationkey (Variables|Default|GetPatrolLocationKey))
  (bind _asenemy_character (Utilities|Casting|CastToEnemyCharacter ControlledPawn)
    (:then
      (Rendering|Debug|DrawDebugSphere (Transformation|GetActorLocation _asenemy_character) _patrolradius 12 "(R=1.000000,G=0.979693,B=0.000000,A=1.000000)" 0.0)
      (Default|SetWalkSpeed _asenemy_character (Variables|Default|GetPatrolSpeed))
      (if (.ReturnValue (AI|Navigation|GetRandomReachablePointinRadius (Transformation|GetActorLocation _asenemy_character) _patrolradius 0 0))
        (AI|BehaviorTree|SetBlackboardValueasVector _patrollocationkey (.RandomLocation (AI|Navigation|GetRandomReachablePointinRadius (Transformation|GetActorLocation _asenemy_character) _patrolradius 0 0)))
        (else
          (AI|BehaviorTree|SetBlackboardValueasVector _patrollocationkey (Transformation|GetActorLocation _asenemy_character))))
      (AI|BehaviorTree|FinishExecute true))
    (:CastFailed
      (AI|BehaviorTree|FinishExecute false))))
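; Enemy AI controller that runs the BT_Enemy behavior tree on possess and feeds perception results into its Blackboard.
; Sensing a Player-tagged actor sets sight and target keys and starts a looping timer that compares distance to the pawn's AttackRange for the in-range key.
; Any other perception update stops that check, clears the in-range key and starts a delay before sight and target are cleared.
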(event OnTargetPerceptionUpdated(AIPerception)
  (params (Actor :type Actor%20Object%20Reference) (Stimulus :type AI%20Stimulus%20Structure))
  (bind _blackboard (Variables|Default|GetBlackboard))
  ;[1 1 1] Perception - sight
  (Variables|Default|SetTargetRef Actor)
  (Utilities|FlowControl|Sequence
    (:then_0
      (if (and (Actor|ActorHasTag Actor "Player") (.bSuccessfullySensed (Utilities|Struct|BreakAIStimulus Stimulus)))
        ;;[1 1 1] See the target?
        (Utilities|Time|ClearandInvalidateTimerbyHandle (Variables|Default|GetLoseSightTimer))
        (AI|Components|Blackboard|SetValueasBool _blackboard (Variables|Default|GetKeyName_HasSight) true)
        (AI|Components|Blackboard|SetValueasObject _blackboard (Variables|Default|GetKeyName_TargetActor) (Variables|Default|GetTargetRef))
        ;;[1 1 1] Has the target in the attack range?
        (bind _returnvalue (Utilities|Time|SetTimerbyEvent (delegate Custom|StartAttackCheck) (Variables|Default|GetAttackCheckInterval) true))
        (Variables|Default|SetAttackCheckTimer _returnvalue)
        (else
          (bind _returnvalue_2 (Utilities|Time|SetTimerbyEvent (delegate Custom|StartLoseSightTimer) (Variables|Default|GetSightTimeLen)))
          (Variables|Default|SetLoseSightTimer _returnvalue_2)
          (AI|Components|Blackboard|SetValueasBool (Variables|Default|GetBlackboard) (Variables|Default|GetKeyName_TargetInRange) false)
          (Utilities|Time|ClearandInvalidateTimerbyHandle (Variables|Default|GetAttackCheckTimer)))))))

(event Custom|StartLoseSightTimer
  (bind _blackboard (Variables|Default|GetBlackboard))
  ;[1 1 1] Perception - sight
  ;;[1 1 1] See the target?
  (AI|Components|Blackboard|SetValueasBool _blackboard (Variables|Default|GetKeyName_HasSight) false)
  (AI|Components|Blackboard|SetValueasObject _blackboard (Variables|Default|GetKeyName_TargetActor) 0))

(event Custom|StartAttackCheck
  (bind _returnvalue (Pawn|GetControlledPawn))
  ;[1 1 1] Perception - sight
  ;;[1 1 1] Has the target in the attack range?
  (bind _asenemy_character_base (Utilities|Casting|CastToEnemyCharacter_Base _returnvalue))
  (AI|Components|Blackboard|SetValueasBool (Variables|Default|GetBlackboard) (Variables|Default|GetKeyName_TargetInRange) (>= (Variables|/Game/Blueprints/EnemyAI/Characters/EnemyCharacter_Base.EnemyCharacter_Base_C|GetAttackRange _asenemy_character_base) (Math|Vector|Distance(Vector) (Transformation|GetActorLocation (Variables|Default|GetTargetRef)) (Transformation|GetActorLocation _returnvalue)))))

(event EventPossess
  (params (PossessedPawn :type Pawn%20Object%20Reference))
  ;[1 1 1] Run the behavior tree
  (AI|RunBehaviorTree "/Game/Blueprints/EnemyAI/BehaviorTree/BT_Enemy.BT_Enemy"))

(fn ConstructionScript)
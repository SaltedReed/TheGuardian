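; Enemy spawner actor that periodically spawns AI enemies inside a box area during battle.
; It binds to the BattleGameMode's battle-start event, then spawns immediately and repeats on a looping timer.
; Each tick counts all world actors of the configured enemy class and, while below the maximum, spawns one at a random point in the box with the enemy behavior tree.
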(event Custom|SpawnEnemy
  (bind _area (Variables|Default|GetArea))
  ;[1 1 1] Spawn enemies
  (bind _outactors (Actor|GetAllActorsOfClass (Variables|Default|GetEnemyType)))
  (if (< (Utilities|Array|Length _outactors) (Variables|Default|GetMaxEnemyCount))
    (AI|SpawnAIFromClass (Variables|Default|GetEnemyType) "/Game/Blueprints/EnemyAI/BehaviorTree/BT_Enemy.BT_Enemy" (Math|Random|RandomPointinBoundingBox (Transformation|GetWorldLocation _area) (Components|Box|GetScaledBoxExtent _area)) "0, 0, 0" false 0)))

(event Custom|StartEnemySpawnTimer
  ;[1 1 1] Init: set enemy-spawn timer
  (Utilities|Time|SetTimerbyFunctionName 0 "SpawnEnemy" (Variables|Default|GetInterval) true)
  (CallFunction|SpawnEnemy))

(event EventBeginPlay
  ;[1 1 1] Init: set enemy-spawn timer
  (bind _asbattle_game_mode (Utilities|Casting|CastToBattleGameMode (Game|GetGameMode)))
  (EventDispatchers|BindEventtoOnBattleStart _asbattle_game_mode (delegate Custom|StartEnemySpawnTimer)))

(fn ConstructionScript)
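; Game mode that runs a timed match: a preparation phase, then a battle phase, then a return to the main menu.
; Each phase pairs a one-second looping countdown that broadcasts remaining time with a one-shot timer that ends it.
; Input is UI-only during preparation and game-and-UI during battle.
; Battle end reverts to UI-only, broadcasts the player's kill and death counts, and loads MainMenuMap after a delay.
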(event Custom|EndBattle
  ;[1 1 1] Timer: battle
  ;;[1 1 1] End battle: input, ui, back to main menu
  (Utilities|FlowControl|Sequence
    (:then_0
      (Input|SetInputModeUIOnly (Game|GetPlayerController 0) 0 "DoNotLock")
      (bind _astg_character (Utilities|Casting|CastToTG_Character (Game|GetPlayerCharacter 0)))
      (Default|CallOnBattleEnd (Variables|/Game/Blueprints/TG_Character.TG_Character_C|GetKillCounts _astg_character) (Variables|/Game/Blueprints/TG_Character.TG_Character_C|GetDeathCounts _astg_character))
      (Utilities|Time|ClearTimerbyFunctionName 0 "CountDownBattle")
      (Utilities|Time|ClearandInvalidateTimerbyHandle (Variables|Default|GetBattleTimer)))
    (:then_1
      (Utilities|FlowControl|Delay 5.0)
      (Game|OpenLevel(byName) "MainMenuMap"))))

(event Custom|EndPreparation
  ;[1 1 1] Timer: preparation before battle
  (Utilities|Time|ClearTimerbyFunctionName 0 "CountDownPrep")
  (CallFunction|SetBattleTimer)
  (Input|SetInputModeGameandUI (Game|GetPlayerController 0) 0 "DoNotLock" true)
  (Default|CallOnBattleStart)
  (Utilities|Time|ClearandInvalidateTimerbyHandle (Variables|Default|GetPrepTimer)))

(event Custom|CountDownPrep
  ;[1 1 1] Timer: preparation before battle
  (bind _output_get (Variables|Default|SetPrepTimeLeft (Math|Float|Max(Float) (- (Variables|Default|GetPrepTimeLeft) 1.0) 0.0)))
  (Default|CallOnPrepCountDownUpdate _output_get))

(event Custom|CountDownBattle
  ;[1 1 1] Timer: battle
  (bind _output_get (Variables|Default|SetBattleTimeLeft (Math|Float|Max(Float) (- (Variables|Default|GetBattleTimeLeft) 1.0) 0.0)))
  (Default|CallOnBattleCountDownUpdate _output_get))

(event Custom|SetPrepTimer
  (bind _preptimelen (Variables|Default|GetPrepTimeLen))
  ;[1 1 1] Timer: preparation before battle
  (Variables|Default|SetPrepTimeLeft _preptimelen)
  (Utilities|Time|SetTimerbyFunctionName 0 "CountDownPrep" 1.0 true)
  (bind _returnvalue (Utilities|Time|SetTimerbyEvent (delegate Custom|EndPreparation) _preptimelen))
  (Variables|Default|SetPrepTimer _returnvalue))

(event Custom|SetBattleTimer
  (bind _battletimelen (Variables|Default|GetBattleTimeLen))
  ;[1 1 1] Timer: battle
  (Variables|Default|SetBattleTimeLeft _battletimelen)
  (Utilities|Time|SetTimerbyFunctionName 0 "CountDownBattle" 1.0 true)
  (bind _returnvalue (Utilities|Time|SetTimerbyEvent (delegate Custom|EndBattle) _battletimelen))
  (Variables|Default|SetBattleTimer _returnvalue))

(event EventBeginPlay
  (Input|SetInputModeUIOnly (Game|GetPlayerController 0) 0 "DoNotLock")
  (CallFunction|SetPrepTimer))

(fn ConstructionScript)